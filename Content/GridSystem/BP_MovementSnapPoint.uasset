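; Grid cell actor for movement on a snap grid, showing hover highlight, edge borders and a translucent grid outline.
; On begin play it traces down for ground and up for obstacles to set validity and occupant, then traces four ways to record valid neighbour cells.
; Valid cells show borders against invalid or missing neighbours, offset for bigger obstacles.
; Dynamic material instances and plane scaling apply the parent grid's styling.
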(event `self.ReceiveBeginPlay`
  ;[0 0.7811 1] Begin play
  (bind _asbp_top_down_controller (cast `/Game/TopDown/Blueprints/BP_TopDownController` (`GameplayStatics.GetPlayerController` 0))
    (:`then`
      (set `self.PlayerControllerRef` _asbp_top_down_controller))
    (:`CastFailed`
      _))
  (`self.C_SetNeighbours&ActorOnIt`)
  (`KismetSystemLibrary.Delay` 0.0)
  (`self.C_InitParameters`))

(event `C_UpdateBorders`
  ;[0.04904 0 1] Border Update
  (`self.FCT_ClearNeighbours`)
  (`self.FCT_CheckIfCellIsValid`)
  (`self.FCT_CheckNearbyCells` "NewEnumerator4"))

(event `C_InitParameters`
  (bind _gridref (`self.GridRef`))
  (bind _gridref_2 (`self.GridRef`))
  ;[1 0.816 0] Parameters init
  ;;[1 1 1] Border parameters init
  (`self.FCT_ModifyBorderColor` (struct))
  (`self.FCT_ModifyBorderOpacity` (`/Game/GridSystem/BP_ScalableGrid.InGameBorderOpacity` _gridref))
  (`self.FCT_ModifyBorderThickness` (`/Game/GridSystem/BP_ScalableGrid.BorderThickness` _gridref))
  ;;[1 1 1] Translucent grid parameters init
  (`self.FCT_ModifyTranslucentGridColor` (struct))
  (`self.FCT_ModifyTranslucentGridOpacity` (`/Game/GridSystem/BP_ScalableGrid.TranslucentGridOpacity` _gridref_2))
  (`self.FCT_ModifyTranslucentGridThickness` (`/Game/GridSystem/BP_ScalableGrid.TranslucentGridThickness` _gridref_2)))

(event `C_SetNeighbours&ActorOnIt`
  ;[1 0.1419 0.9555] Check if cells is usable & set neighbours for movement
  (`self.FCT_CheckIfCellIsValid`)
  (`KismetSystemLibrary.Delay` 0.0)
  (`self.FCT_CheckNearbyCells` "NewEnumerator4"))

(event `C_HoverSquare`
  ;[0.1437 1 0.2378] Hover & Unhover square
  (`self.Fct_ShowTargetedPlane`))

(event `C_UnhoverSquare`
  ;[0.1437 1 0.2378] Hover & Unhover square
  (`self.Fct_HidePlane`))

(event `C_ShowBorders`
  ;[1 0.4908 0.1101] Show borders
  (`self.ActorOnIt`
    (:`then`)
    (:`else`
      (`self.FCT_SetBorders`))))

(fn `Fct_BorderDisplay`
  (params (Direction :type "/Game/GridSystem/E_Directions Enum" :default "NewEnumerator0") (NeedToMove :type Boolean) (`NeedToDisplay?` :type Boolean))
  (locals (LocalNeedToDisplay :type Boolean) (LocalNeedToMove :type Boolean))
  (bind _planes (`self.PlaneS`))
  (bind _planee (`self.PlaneE`))
  (bind _planew (`self.PlaneW`))
  (bind _planen (`self.PlaneN`))
  (bind (_returnvalue_x _returnvalue_y _returnvalue_z) (`KismetMathLibrary.BreakVector` (`SceneComponent.K2_GetComponentLocation` _planew)))
  (bind (_returnvalue_x_2 _returnvalue_y_2 _returnvalue_z_2) (`KismetMathLibrary.BreakVector` (`SceneComponent.K2_GetComponentLocation` _planen)))
  (bind (_returnvalue_x_3 _returnvalue_y_3 _returnvalue_z_3) (`KismetMathLibrary.BreakVector` (`SceneComponent.K2_GetComponentLocation` _planes)))
  (bind (_returnvalue_x_4 _returnvalue_y_4 _returnvalue_z_4) (`KismetMathLibrary.BreakVector` (`SceneComponent.K2_GetComponentLocation` _planee)))
  (set `local.LocalNeedToMove` NeedToMove)
  (set `local.LocalNeedToDisplay` `NeedToDisplay?`)
  (switch `/Game/GridSystem/E_Directions` Direction
    (:`NewEnumerator0`
      ;[0 0.004391 0.3564] Toggle visibility North border
      (if (`local.LocalNeedToMove`)
        (`SceneComponent.SetRelativeScale3D` _planen (`self.N&SBorderBiggerScale`))
        (`SceneComponent.K2_SetWorldLocation` _planen (`KismetMathLibrary.MakeVector` (- _returnvalue_x_2 (`self.BorderOffset`)) _returnvalue_y_2 _returnvalue_z_2) false false)
        (else
          (`SceneComponent.SetRelativeScale3D` _planen (`self.N&SBorderBaseScale`))))
      (if (`local.LocalNeedToDisplay`)
        (`SceneComponent.SetVisibility` _planen true false)
        (else
          (`SceneComponent.SetVisibility` _planen false false))))
    (:`NewEnumerator1`
      ;[1 0.4852 0.08228] Toggle visibility South border
      (if (`local.LocalNeedToMove`)
        (`SceneComponent.SetRelativeScale3D` _planes (`self.N&SBorderBiggerScale`))
        (`SceneComponent.K2_SetWorldLocation` _planes (`KismetMathLibrary.MakeVector` (+ _returnvalue_x_3 (`self.BorderOffset`)) _returnvalue_y_3 _returnvalue_z_3) false false)
        (else
          (`SceneComponent.SetRelativeScale3D` _planes (`self.N&SBorderBaseScale`))))
      (if (`local.LocalNeedToDisplay`)
        (`SceneComponent.SetVisibility` _planes true false)
        (else
          (`SceneComponent.SetVisibility` _planes false false))))
    (:`NewEnumerator2`
      ;[0 1 0.06663] Toggle visibility South border
      (if (`local.LocalNeedToMove`)
        (`SceneComponent.SetRelativeScale3D` _planee (`self.E&WBorderBiggerScale`))
        (`SceneComponent.K2_SetWorldLocation` _planee (`KismetMathLibrary.MakeVector` _returnvalue_x_4 (- _returnvalue_y_4 (`self.BorderOffset`)) _returnvalue_z_4) false false)
        (else
          (`SceneComponent.SetRelativeScale3D` _planee (`self.E&WBorderBaseScale`))))
      (if (`local.LocalNeedToDisplay`)
        (`SceneComponent.SetVisibility` _planee true false)
        (else
          (`SceneComponent.SetVisibility` _planee false false))))
    (:`NewEnumerator3`
      ;[1 0 0.9301] Toggle visibility South border
      (if (`local.LocalNeedToMove`)
        (`SceneComponent.SetRelativeScale3D` _planew (`self.E&WBorderBiggerScale`))
        (`SceneComponent.K2_SetWorldLocation` _planew (`KismetMathLibrary.MakeVector` _returnvalue_x (+ _returnvalue_y (`self.BorderOffset`)) _returnvalue_z) false false)
        (else
          (`SceneComponent.SetRelativeScale3D` _planew (`self.E&WBorderBaseScale`))))
      (if (`local.LocalNeedToDisplay`)
        (`SceneComponent.SetVisibility` _planew true false)
        (else
          (`SceneComponent.SetVisibility` _planew false false)))))
  (return))

(fn `FCT_ChangePlaneColor`
  (params (`BecomeRed?` :type Boolean))
  (bind _targetedplane (`self.TargetedPlane`))
  (if `BecomeRed?`
    (`PrimitiveComponent.SetMaterial` _targetedplane 0 null)
    (else
      (`PrimitiveComponent.SetMaterial` _targetedplane 0 null)))
  (return))

(fn `FCT_CheckIfCellIsValid`
  (bind _linetraceorigin (`self.LineTraceOrigin`))
  (bind _returnvalue (`SceneComponent.K2_GetComponentLocation` (`self.LineTraceOrigin`)))
  (bind (_returnvalue_x _returnvalue_y _returnvalue_z) (`KismetMathLibrary.BreakVector` (`SceneComponent.K2_GetComponentLocation` _linetraceorigin)))
  ;[0.2812 0.1164 0.03943] Check if there is a ground under the cell
  (bind _outhit (`KismetSystemLibrary.LineTraceSingle` :`Start` (`SceneComponent.K2_GetComponentLocation` _linetraceorigin) :`End` (`KismetMathLibrary.MakeVector` _returnvalue_x _returnvalue_y (- _returnvalue_z 400.0)) :`TraceChannel` "TraceTypeQuery3" :`bTraceComplex` true :`DrawTime` 10.0))
  (if (`GameplayStatics.BreakHitResult` _outhit)
    (set `self.AmIValid?` true)
    (else
      (set `self.AmIValid?` false)))
  ;[1 0 0.06854] Check if there is an obstacle on the cell
  (bind _outhit_2 (`KismetSystemLibrary.SphereTraceSingle` _returnvalue (+ _returnvalue (0.0 0.0 150.0)) 20.0 "TraceTypeQuery3"))
  (bind _asbp_obstacle_parent (cast `/Game/GridSystem/BP_ObstacleParent` (`.HitActor` (`GameplayStatics.BreakHitResult` _outhit_2)))
    (:`then`
      (set `self.AmIValid?` false)
      (`self.FCT_SetActorOnIt` _asbp_obstacle_parent)
      (`KismetArrayLibrary.Array_Add` (`/Game/GridSystem/BP_ObstacleParent.SquareOnREF` _asbp_obstacle_parent) self))
    (:`CastFailed`
      (if (`self.AmIValid?`)
        (set `self.AmIValid?` true))))
  (return))

(fn `FCT_CheckNearbyCells`
  (params (Direction :type "/Game/GridSystem/E_Directions Enum" :default "NewEnumerator0"))
  (locals (NewLocalVar :type "Array of HitResult Structure") (LocalNeedBorderManagement :type Boolean))
  (bind _linetraceorigin (`self.LineTraceOrigin`))
  (bind _linetraceorigin_2 (`self.LineTraceOrigin`))
  (bind _linetraceorigin_3 (`self.LineTraceOrigin`))
  (bind _linetraceorigin_4 (`self.LineTraceOrigin`))
  (bind _returnvalue (`SceneComponent.K2_GetComponentLocation` _linetraceorigin_4))
  (bind _returnvalue_2 (`SceneComponent.K2_GetComponentLocation` _linetraceorigin_3))
  (bind _returnvalue_3 (`SceneComponent.K2_GetComponentLocation` _linetraceorigin))
  (bind _returnvalue_4 (`SceneComponent.K2_GetComponentLocation` _linetraceorigin_2))
  (switch `/Game/GridSystem/E_Directions` Direction
    (:`NewEnumerator0`
      ;[0 0.004391 0.3564] Set visibility North Border
      (bind _outhit (`KismetSystemLibrary.LineTraceSingle` :`Start` _returnvalue_4 :`End` (+ _returnvalue_4 (* (`SceneComponent.GetForwardVector` _linetraceorigin_2) 200.0)) :`TraceChannel` "TraceTypeQuery3" :`bTraceComplex` true :`DrawTime` 1.0 :!label _label))
      (bind _asbp_movement_snap_point (cast `/Game/GridSystem/BP_MovementSnapPoint` (`.HitActor` (`GameplayStatics.BreakHitResult` _outhit)))
        (:`then`
          (if (`/Game/GridSystem/BP_MovementSnapPoint.AmIValid?` _asbp_movement_snap_point)
            (`KismetArrayLibrary.Array_AddUnique` (`self.Neighbours`) (make `/Game/GridSystem/F_Neihbours` _asbp_movement_snap_point))
            (elif (`self.AmIValid?`)
              (bind _actoronit (`/Game/GridSystem/BP_MovementSnapPoint.ActorOnIt` _asbp_movement_snap_point))
              (if (`KismetSystemLibrary.IsValid` _actoronit)
                (`self.MA_ObstacleCheck` _actoronit
                  (:`Bigger`
                    (`self.Fct_BorderDisplay` "NewEnumerator0" true true :!label _label_2))
                  (:`Normal`
                    (`self.Fct_BorderDisplay` "NewEnumerator0" false true :!label _label_3))
                  (:`CastFailed`
                    (goto _label_3)))
                (else
                  (goto _label_3))))))
        (:`CastFailed`
          (if (`self.AmIValid?`)
            (`self.MA_ObstacleCheck` (`.HitActor` (`GameplayStatics.BreakHitResult` _outhit))
              (:`Bigger`
                (goto _label_2))
              (:`Normal`
                (goto _label_3))
              (:`CastFailed`
                (goto _label_3)))))))
    (:`NewEnumerator1`
      ;[1 0.4852 0.08228] Set visibility South Border
      (bind _outhit_2 (`KismetSystemLibrary.LineTraceSingle` :`Start` _returnvalue :`End` (+ _returnvalue (* (`SceneComponent.GetForwardVector` _linetraceorigin_4) -200.0)) :`TraceChannel` "TraceTypeQuery3" :`DrawTime` 1.0 :!label _label_4))
      (bind _asbp_movement_snap_point_2 (cast `/Game/GridSystem/BP_MovementSnapPoint` (`.HitActor` (`GameplayStatics.BreakHitResult` _outhit_2)))
        (:`then`
          (if (`/Game/GridSystem/BP_MovementSnapPoint.AmIValid?` _asbp_movement_snap_point_2)
            (`KismetArrayLibrary.Array_AddUnique` (`self.Neighbours`) (make `/Game/GridSystem/F_Neihbours` _asbp_movement_snap_point_2 "NewEnumerator1"))
            (elif (`self.AmIValid?`)
              (bind _actoronit_2 (`/Game/GridSystem/BP_MovementSnapPoint.ActorOnIt` _asbp_movement_snap_point_2))
              (if (`KismetSystemLibrary.IsValid` _actoronit_2)
                (`self.MA_ObstacleCheck` _actoronit_2
                  (:`Bigger`
                    (`self.Fct_BorderDisplay` "NewEnumerator1" true true :!label _label_5))
                  (:`Normal`
                    (`self.Fct_BorderDisplay` "NewEnumerator1" false true :!label _label_6))
                  (:`CastFailed`
                    (goto _label_6)))
                (else
                  (goto _label_6))))))
        (:`CastFailed`
          (if (`self.AmIValid?`)
            (`self.MA_ObstacleCheck` (`.HitActor` (`GameplayStatics.BreakHitResult` _outhit_2))
              (:`Bigger`
                (goto _label_5))
              (:`Normal`
                (goto _label_6))
              (:`CastFailed`
                (goto _label_6)))))))
    (:`NewEnumerator2`
      ;[0 1 0.06663] Set visibility East Border
      (bind _outhit_3 (`KismetSystemLibrary.LineTraceSingle` _returnvalue_3 (+ _returnvalue_3 (* (`SceneComponent.GetRightVector` _linetraceorigin) 200.0)) "TraceTypeQuery3" :!label _label_7))
      (bind _asbp_movement_snap_point_3 (cast `/Game/GridSystem/BP_MovementSnapPoint` (`.HitActor` (`GameplayStatics.BreakHitResult` _outhit_3)))
        (:`then`
          (if (`/Game/GridSystem/BP_MovementSnapPoint.AmIValid?` _asbp_movement_snap_point_3)
            (`KismetArrayLibrary.Array_AddUnique` (`self.Neighbours`) (make `/Game/GridSystem/F_Neihbours` _asbp_movement_snap_point_3))
            (elif (`self.AmIValid?`)
              (bind _actoronit_3 (`/Game/GridSystem/BP_MovementSnapPoint.ActorOnIt` _asbp_movement_snap_point_3))
              (if (`KismetSystemLibrary.IsValid` _actoronit_3)
                (`self.MA_ObstacleCheck` _actoronit_3
                  (:`Bigger`
                    (`self.Fct_BorderDisplay` "NewEnumerator2" true true :!label _label_8))
                  (:`Normal`
                    (`self.Fct_BorderDisplay` "NewEnumerator2" false true :!label _label_9))
                  (:`CastFailed`
                    (goto _label_9)))
                (else
                  (goto _label_9))))))
        (:`CastFailed`
          (if (`self.AmIValid?`)
            (`self.MA_ObstacleCheck` (`.HitActor` (`GameplayStatics.BreakHitResult` _outhit_3))
              (:`Bigger`
                (goto _label_8))
              (:`Normal`
                (goto _label_9))
              (:`CastFailed`
                (goto _label_9)))))))
    (:`NewEnumerator3`
      ;[1 0 0.9301] Set visibility West Border
      (bind _outhit_4 (`KismetSystemLibrary.LineTraceSingle` :`Start` _returnvalue_2 :`End` (+ _returnvalue_2 (* (`SceneComponent.GetRightVector` _linetraceorigin_3) -200.0)) :`TraceChannel` "TraceTypeQuery3" :`DrawTime` 1.0 :!label _label_10))
      (bind _asbp_movement_snap_point_4 (cast `/Game/GridSystem/BP_MovementSnapPoint` (`.HitActor` (`GameplayStatics.BreakHitResult` _outhit_4)))
        (:`then`
          (if (`/Game/GridSystem/BP_MovementSnapPoint.AmIValid?` _asbp_movement_snap_point_4)
            (`KismetArrayLibrary.Array_AddUnique` (`self.Neighbours`) (make `/Game/GridSystem/F_Neihbours` _asbp_movement_snap_point_4))
            (elif (`self.AmIValid?`)
              (bind _actoronit_4 (`/Game/GridSystem/BP_MovementSnapPoint.ActorOnIt` _asbp_movement_snap_point_4))
              (if (`KismetSystemLibrary.IsValid` _actoronit_4)
                (`self.MA_ObstacleCheck` _actoronit_4
                  (:`Bigger`
                    (`self.Fct_BorderDisplay` "NewEnumerator3" true true :!label _label_11))
                  (:`Normal`
                    (`self.Fct_BorderDisplay` "NewEnumerator3" false true :!label _label_12))
                  (:`CastFailed`
                    (goto _label_12)))
                (else
                  (goto _label_12))))))
        (:`CastFailed`
          (if (`self.AmIValid?`)
            (`self.MA_ObstacleCheck` (`.HitActor` (`GameplayStatics.BreakHitResult` _outhit_4))
              (:`Bigger`
                (goto _label_11))
              (:`Normal`
                (goto _label_12))
              (:`CastFailed`
                (goto _label_12)))))))
    (:`NewEnumerator4`
      (`|ExecutionSequence`
        (:`then_0`
          (goto _label))
        (:`then_1`
          (goto _label_4))
        (:`then_2`
          (goto _label_7))
        (:`then_3`
          (goto _label_10))))))

(fn `FCT_ClearNeighbours`
  (`KismetArrayLibrary.Array_Clear` (`self.Neighbours`))
  (return))

(fn `Fct_HidePlane`
  (`SceneComponent.SetVisibility` (`self.TargetedPlane`) false false)
  (return))

(fn `FCT_ModifyBorderColor`
  (params (NewColor :type "LinearColor Structure"))
  (if (`self.BorderMatInit?`)
    (`MaterialInstanceDynamic.SetVectorParameterValue` (`self.BorderMatInstance`) "Color" NewColor)
    (else
      (bind _returnvalue (`KismetMaterialLibrary.CreateDynamicMaterialInstance` "/Game/GridSystem/M_Border_Mat.M_Border_Mat"))
      (bind _output_get (set `self.BorderMatInstance` _returnvalue))
      (for _array_element (`|MakeArray` (`self.PlaneN`) (`self.PlaneS`) (`self.PlaneE`) (`self.PlaneW`))
        (`PrimitiveComponent.SetMaterial` _array_element 0 _output_get))
      (`MaterialInstanceDynamic.SetVectorParameterValue` (`self.BorderMatInstance`) "Color" (`/Game/GridSystem/BP_ScalableGrid.InGameBorderColor` (`self.GridRef`)))
      (set `self.BorderMatInit?` true))))

(fn `FCT_ModifyBorderOpacity`
  (params (NewOpacity :type "Float (double-precision)"))
  (if (`self.BorderMatInit?`)
    (`MaterialInstanceDynamic.SetScalarParameterValue` (`self.BorderMatInstance`) "Opacity" NewOpacity)
    (else
      (bind _returnvalue (`KismetMaterialLibrary.CreateDynamicMaterialInstance` "/Game/GridSystem/M_Border_Mat.M_Border_Mat"))
      (bind _output_get (set `self.BorderMatInstance` _returnvalue))
      (for _array_element (`|MakeArray` (`self.PlaneN`) (`self.PlaneS`) (`self.PlaneE`) (`self.PlaneW`))
        (`PrimitiveComponent.SetMaterial` _array_element 0 _output_get))
      (`MaterialInstanceDynamic.SetScalarParameterValue` (`self.BorderMatInstance`) "Opacity" (`/Game/GridSystem/BP_ScalableGrid.InGameBorderOpacity` (`self.GridRef`)))
      (set `self.BorderMatInit?` true))))

(fn `FCT_ModifyBorderThickness`
  (params (NewThickness :type "Float (double-precision)"))
  (bind _returnvalue (* (`self.MaxBordersThickness`) NewThickness))
  (bind (_relativescale3d_x _relativescale3d_y _relativescale3d_z) (`KismetMathLibrary.BreakVector` (`SceneComponent.RelativeScale3D` (`self.PlaneW`))))
  (bind (_relativescale3d_x_2 _relativescale3d_y_2 _relativescale3d_z_2) (`KismetMathLibrary.BreakVector` (`SceneComponent.RelativeScale3D` (`self.PlaneS`))))
  ;[1 1 1] Modify scale for N & S part
  (`SceneComponent.SetRelativeScale3D` (`self.PlaneN`) (`KismetMathLibrary.MakeVector` _returnvalue _relativescale3d_y_2 _relativescale3d_z_2))
  (`SceneComponent.SetRelativeScale3D` (`self.PlaneS`) (`KismetMathLibrary.MakeVector` _returnvalue _relativescale3d_y_2 _relativescale3d_z_2))
  ;[1 1 1] Same for S & W part
  (`SceneComponent.SetRelativeScale3D` (`self.PlaneE`) (`KismetMathLibrary.MakeVector` _relativescale3d_x _returnvalue _relativescale3d_z))
  (`SceneComponent.SetRelativeScale3D` (`self.PlaneW`) (`KismetMathLibrary.MakeVector` _relativescale3d_x _returnvalue _relativescale3d_z))
  (return))

(fn `FCT_ModifyTranslucentGridColor`
  (params (NewColor :type "LinearColor Structure"))
  (if (`self.TranslucentGridMatInit?`)
    (`MaterialInstanceDynamic.SetVectorParameterValue` (`self.TranslucentGridMatInstance`) "Color" NewColor)
    (else
      (bind _returnvalue (`KismetMaterialLibrary.CreateDynamicMaterialInstance` "/Game/GridSystem/M_TranslucentGrid_Mat.M_TranslucentGrid_Mat"))
      (bind _output_get (set `self.TranslucentGridMatInstance` _returnvalue))
      (for _array_element (`|MakeArray` (`self.TranslucentGridN`) (`self.TranslucentGridS`) (`self.TranslucentGridE`) (`self.TranslucentGridW`))
        (`PrimitiveComponent.SetMaterial` _array_element 0 _output_get))
      (`MaterialInstanceDynamic.SetVectorParameterValue` (`self.TranslucentGridMatInstance`) "Color" (`/Game/GridSystem/BP_ScalableGrid.TranslucentGridColor` (`self.GridRef`)))
      (set `self.TranslucentGridMatInit?` true))))

(fn `FCT_ModifyTranslucentGridOpacity`
  (params (NewOpacity :type "Float (double-precision)"))
  (if (`self.TranslucentGridMatInit?`)
    (`MaterialInstanceDynamic.SetScalarParameterValue` (`self.TranslucentGridMatInstance`) "Opacity" NewOpacity)
    (else
      (bind _returnvalue (`KismetMaterialLibrary.CreateDynamicMaterialInstance` "/Game/GridSystem/M_TranslucentGrid_Mat.M_TranslucentGrid_Mat"))
      (bind _output_get (set `self.TranslucentGridMatInstance` _returnvalue))
      (for _array_element (`|MakeArray` (`self.TranslucentGridN`) (`self.TranslucentGridS`) (`self.TranslucentGridE`) (`self.TranslucentGridW`))
        (`PrimitiveComponent.SetMaterial` _array_element 0 _output_get))
      (`MaterialInstanceDynamic.SetScalarParameterValue` (`self.TranslucentGridMatInstance`) "Opacity" (`/Game/GridSystem/BP_ScalableGrid.TranslucentGridOpacity` (`self.GridRef`)))
      (set `self.TranslucentGridMatInit?` true))))

(fn `FCT_ModifyTranslucentGridThickness`
  (params (NewThickness :type "Float (double-precision)"))
  (bind _translucentgridn (`self.TranslucentGridN`))
  (bind _translucentgride (`self.TranslucentGridE`))
  (bind _returnvalue (* (`self.MaxTranslucentGridThickness`) NewThickness))
  (bind (_relativescale3d_x _relativescale3d_y _relativescale3d_z) (`KismetMathLibrary.BreakVector` (`SceneComponent.RelativeScale3D` _translucentgride)))
  (bind (_relativescale3d_x_2 _relativescale3d_y_2 _relativescale3d_z_2) (`KismetMathLibrary.BreakVector` (`SceneComponent.RelativeScale3D` _translucentgridn)))
  ;[1 1 1] Modify scale for N & S part
  (`SceneComponent.SetRelativeScale3D` _translucentgridn (`KismetMathLibrary.MakeVector` _returnvalue _relativescale3d_y_2 _relativescale3d_z_2))
  (`SceneComponent.SetRelativeScale3D` (`self.TranslucentGridS`) (`KismetMathLibrary.MakeVector` _returnvalue _relativescale3d_y_2 _relativescale3d_z_2))
  ;[1 1 1] Same for S & W part
  (`SceneComponent.SetRelativeScale3D` _translucentgride (`KismetMathLibrary.MakeVector` _relativescale3d_x _returnvalue _relativescale3d_z))
  (`SceneComponent.SetRelativeScale3D` (`self.TranslucentGridW`) (`KismetMathLibrary.MakeVector` _relativescale3d_x _returnvalue _relativescale3d_z))
  (return))

(fn `FCT_SetActorOnIt`
  (params (Actor :type "Actor Object Reference"))
  (set `self.ActorOnIt` Actor)
  (`self.FCT_ChangePlaneColor` true)
  (return))

(fn `FCT_SetBorders`
  (for _array_element (`self.Neighbours`)
    (`/Engine/EditorBlueprintResources/StandardMacros.IsValid` (`/Game/GridSystem/BP_MovementSnapPoint.ActorOnIt` (break `/Game/GridSystem/F_Neihbours` _array_element))
      (:`Is Valid`
        (`self.Fct_BorderDisplay` (`.Side_8_10B557694281E995C61A068DCB769135` (break `/Game/GridSystem/F_Neihbours` _array_element)) false true))))
  (return))

(fn `Fct_ShowTargetedPlane`
  (`SceneComponent.SetVisibility` (`self.TargetedPlane`) true false)
  (return))

(fn `FCT_UnsetActorOniT`
  (set `self.ActorOnIt` null)
  (`self.FCT_ChangePlaneColor` false))

(fn `UserConstructionScript`)