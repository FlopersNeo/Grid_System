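; Scalable grid actor that builds a field of BP_MovementSnapPoint cells as child actors, sized by cell size and grid dimensions.
; The construction script clears and rebuilds the cells, using reduced dimensions when NeedToMoveGrid is set, then caches them in CellsArray with a back-reference to the grid.
; It relays border updates to every cell and sets translucent edge visibility on valid cells, applied at BeginPlay from the TranslucentGrid flag.
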(event `C_UpdateBorders`
  ;[1 1 1] Border Update
  (for _array_element (`self.CellsArray`)
    (`/Game/GridSystem/BP_MovementSnapPoint.C_UpdateBorders` _array_element)))

(event `self.ReceiveBeginPlay`
  ;[0 0.8586 1] Begin play
  (if (`self.TranslucentGrid?`)
    (`self.FCT_OrderTranslucentGrid` true)
    (else
      (`self.FCT_OrderTranslucentGrid` false))))

(fn `FCT_BorderUpdate`
  (for _array_element (`self.CellsArray`)
    (set `/Game/GridSystem/BP_MovementSnapPoint.NeedBorderUpdate?` true _array_element))
  (return))

(fn `Fct_ClearGrid`
  (bind _cellsarray (`self.CellsArray`))
  (for _array_element _cellsarray
    (if (`KismetSystemLibrary.IsValid` _array_element)
      (`self.K2_DestroyActor` _array_element)))
  (`KismetArrayLibrary.Array_Clear` _cellsarray)
  (return))

(fn `Fct_InitGrid`
  (locals (SpawnPosition :type "Vector Structure"))
  (bind _boxgridsize (`self.BoxGridSize`))
  (bind _boxgridsize_2 (`self.BoxGridSize`))
  (bind _returnvalue (/ (`self.BoxGridSize`) 2.0))
  (bind _returnvalue_2 (/ (`self.BoxGridSize`) 2.0))
  (`self.Fct_ClearGrid`)
  (set `self.HaveCreatedGrid?` true)
  (if (`self.NeedToMoveGrid?`)
    ;[0.4574 0.9701 1] Spawn reduced grid
    (for _index (range (`self.ReducedGridSizeX`))
      (for _index_2 (range (`self.ReducedGridSizeY`))
        (bind _returnvalue_3 (`AddComponent|NODE_AddChildActorComponent-3` :`RelativeTransform` (`KismetMathLibrary.MakeTransform` (`KismetMathLibrary.MakeVector` (+ _returnvalue_2 (* _index_2 _boxgridsize_2)) (+ _returnvalue_2 (* _index _boxgridsize_2)) (`self.BaseGridHeight`)))))
        (`ChildActorComponent.SetChildActorClass` _returnvalue_3 "/Game/GridSystem/BP_MovementSnapPoint.BP_MovementSnapPoint_C")))
    (else
      ;[0 0.9424 1] Spawn grid
      (for _index_3 (range (`self.GridSizeX`))
        (for _index_4 (range (`self.GridSizeY`))
          (bind _returnvalue_4 (`AddComponent|NODE_AddChildActorComponent-2` :`RelativeTransform` (`KismetMathLibrary.MakeTransform` (`KismetMathLibrary.MakeVector` (+ _returnvalue (* _index_4 _boxgridsize)) (+ _returnvalue (* _index_3 _boxgridsize)) (`self.BaseGridHeight`)))))
          (`ChildActorComponent.SetChildActorClass` _returnvalue_4 "/Game/GridSystem/BP_MovementSnapPoint.BP_MovementSnapPoint_C")))))
  ;[0.599 0 1] Fill cells array
  (for _array_element (`self.GetAllChildActors` false)
    (bind _asbp_movement_snap_point (cast `/Game/GridSystem/BP_MovementSnapPoint` _array_element))
    (set `/Game/GridSystem/BP_MovementSnapPoint.GridRef` self _asbp_movement_snap_point)
    (`KismetArrayLibrary.Array_Add` (`self.CellsArray`) _asbp_movement_snap_point))
  (set `self.HaveCreatedGrid?` true)
  (return))

(fn `FCT_OrderTranslucentGrid`
  (params (Value :type Boolean))
  (if Value
    (for _array_element (`self.CellsArray`)
      (if (`/Game/GridSystem/BP_MovementSnapPoint.AmIValid?` _array_element)
        (`SceneComponent.SetVisibility` (`/Game/GridSystem/BP_MovementSnapPoint.TranslucentGridN` _array_element) true true)
        (`SceneComponent.SetVisibility` (`/Game/GridSystem/BP_MovementSnapPoint.TranslucentGridS` _array_element) true true)
        (`SceneComponent.SetVisibility` (`/Game/GridSystem/BP_MovementSnapPoint.TranslucentGridE` _array_element) true true)
        (`SceneComponent.SetVisibility` (`/Game/GridSystem/BP_MovementSnapPoint.TranslucentGridW` _array_element) true true)))
    (return)
    (else
      (for _array_element_2 (`self.CellsArray`)
        (if (`/Game/GridSystem/BP_MovementSnapPoint.AmIValid?` _array_element_2)
          (`SceneComponent.SetVisibility` (`/Game/GridSystem/BP_MovementSnapPoint.TranslucentGridN` _array_element_2) false true)
          (`SceneComponent.SetVisibility` (`/Game/GridSystem/BP_MovementSnapPoint.TranslucentGridS` _array_element_2) false true)
          (`SceneComponent.SetVisibility` (`/Game/GridSystem/BP_MovementSnapPoint.TranslucentGridE` _array_element_2) false true)
          (`SceneComponent.SetVisibility` (`/Game/GridSystem/BP_MovementSnapPoint.TranslucentGridW` _array_element_2) false true)))
      (return))))

(fn `UserConstructionScript`
  ;[0 0.8766 1] Init Grid on placement in levels
  (`self.Fct_InitGrid`))